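; Melee sword actor that snaps to a socket on its MainCharacter's mesh and handles hits on characters and other swords.
; BoxD overlaps send damage to characters or interrupt the opposing sword's attack, stopping their own attack and shrinking then re-extending the box when in attack mode.
; BoxS overlaps sphere-trace along the blade and forward the hit for reactions, using DoOnce gates with delayed resets against repeats.
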(event OnComponentBeginOverlap(BoxD)
  (params (OverlappedComponent :type Primitive%20Component%20Object%20Reference) (OtherActor :type Actor%20Object%20Reference) (OtherComp :type Primitive%20Component%20Object%20Reference) (OtherBodyIndex :type Integer) (bFromSweep :type Boolean) (SweepResult :type Hit%20Result%20Structure%20%28by%20ref%29))
  (bind _hitactor (Variables|Default|GetHitActor))
  (bind _actor (CallFunction|IgnoreSelf self OtherActor))
  (bind _assword (Utilities|Casting|CastToSword _actor)
    (:then
      (Default|Damage _assword SweepResult)
      (if (Variables|/Game/Mannequin/Animations/Main_ABP.Main_ABP_C|GetAttackMode (Variables|/Game/Blueprints/MainCharacter.MainCharacter_C|GetAnimReference (Variables|Default|GetMainCharacter)))
        (Default|StopAttack (Variables|Default|GetMainCharacter))
        (CallFunction|UpdateBox)))
    (:CastFailed
      (Utilities|Casting|CastToMainCharacter _hitactor)
      (Class|MainInterface|Damage(Message) _hitactor SweepResult (Variables|Default|GetDamageValue) (Components|GetOwner) self)
      (if (Variables|/Game/Mannequin/Animations/Main_ABP.Main_ABP_C|GetAttackMode (Variables|/Game/Blueprints/MainCharacter.MainCharacter_C|GetAnimReference (Variables|Default|GetMainCharacter)))
        (Default|StopAttack (Variables|Default|GetMainCharacter))
        (CallFunction|UpdateBox)))))

(event OnComponentEndOverlap(BoxD)
  (params (OverlappedComponent :type Primitive%20Component%20Object%20Reference) (OtherActor :type Actor%20Object%20Reference) (OtherComp :type Primitive%20Component%20Object%20Reference) (OtherBodyIndex :type Integer))
  (if (Variables|/Game/Mannequin/Animations/Main_ABP.Main_ABP_C|GetAttackMode (Variables|/Game/Blueprints/MainCharacter.MainCharacter_C|GetAnimReference (Variables|Default|GetMainCharacter)))
    (Default|StopAttack (Variables|Default|GetMainCharacter))))

(event OnComponentBeginOverlap(BoxS)
  (params (OverlappedComponent :type Primitive%20Component%20Object%20Reference) (OtherActor :type Actor%20Object%20Reference) (OtherComp :type Primitive%20Component%20Object%20Reference) (OtherBodyIndex :type Integer) (bFromSweep :type Boolean) (SweepResult :type Hit%20Result%20Structure%20%28by%20ref%29))
  (bind _actor (CallFunction|IgnoreSelf self OtherActor))
  (bind _asmain_character (Utilities|Casting|CastToMainCharacter _actor)
    (:then
      (Utilities|FlowControl|DoOnce false
        (:Completed
          (bind _outhit (CallFunction|SwordLineTrace))
          (Default|HitResult _asmain_character _outhit)
          (Utilities|FlowControl|Delay 0.4)
          (CallFunction|ResetHit))))
    (:CastFailed
      (Utilities|FlowControl|DoOnce false
        (:Completed
          (bind _assword (Utilities|Casting|CastToSword (Variables|Default|GetHitActor)))
          (bind _outhit_2 (CallFunction|SwordLineTrace))
          (Default|HitResult _assword _outhit_2)
          (Utilities|FlowControl|Delay 0.1)
          (CallFunction|ResetSword))))))

(event OnComponentEndOverlap(BoxS)
  (params (OverlappedComponent :type Primitive%20Component%20Object%20Reference) (OtherActor :type Actor%20Object%20Reference) (OtherComp :type Primitive%20Component%20Object%20Reference) (OtherBodyIndex :type Integer))
  (CallFunction|IgnoreSelf self OtherActor))

(event Custom|UpdateBox
  (Components|MoveComponentTo (Variables|Default|GetBoxD) "0, 0,-60.000000" "0, 0, 0" false false 0.4 false)
  (Transformation|SetWorldScale3D (Variables|Default|GetBoxD) "0.025000,0.070000,0.070000")
  (Utilities|FlowControl|Delay 0.0)
  (Components|MoveComponentTo (Variables|Default|GetBoxD) "0, 0,60.000000" "0, 0, 0" false false 0.4 false)
  (Transformation|SetWorldScale3D (Variables|Default|GetBoxD) "0.025000,0.070000,1.300000"))

(event Custom|AttachSword
  (Transformation|AttachComponentToComponent (Variables|Default|GetAttachment) (Variables|/Script/Engine.Character|GetMesh (Variables|Default|GetMainCharacter)) (Variables|Default|GetSocket%20Name) "SnapToTarget" "SnapToTarget" "SnapToTarget" true))

(event Custom|ResetHit
  (Utilities|FlowControl|DoOnce false) ; enters at Reset
)

(event Custom|ResetSword
  (Utilities|FlowControl|DoOnce false) ; enters at Reset
)

(event EventBeginPlay
  (CallFunction|AttachSword))

(event EventHitResult
  (params (HitResult :type Hit%20Result%20Structure))
  (bind _hitactor (Collision|BreakHitResult HitResult))
  (if (== _hitactor self)
    (Default|HitReaction (Variables|Default|GetMainCharacter) "hand_r")
    (else
      (bind _assword (Utilities|Casting|CastToSword _hitactor))
      (Default|HitReaction (Variables|Sword_C|GetMainCharacter _assword) "hand_r"))))

(event EventDamage
  (params (HitResult :type Hit%20Result%20Structure) (Damage :type Integer) (DamageOwner :type Actor%20Object%20Reference) (DamageCauser :type Actor%20Object%20Reference))
  (Default|StopAttack (Variables|Default|GetMainCharacter)))

(fn ConstructionScript)

(fn IgnoreSelf
  (params (HitActor :type Actor%20Object%20Reference))
  (Variables|Default|SetHitActor HitActor)
  (if (and (!= (Variables|Default|GetMainCharacter) (Variables|Default|GetHitActor)) (!= (Variables|Default|GetHitActor) self))
    (return (Variables|Default|GetHitActor))))

(fn SwordLineTrace
  (bind _boxs (Variables|Default|GetBoxS))
  (bind _returnvalue (Transformation|GetWorldLocation _boxs))
  (bind _outhit (Collision|SphereTraceByChannel (+ (* (Math|Vector|GetUpVector _boxs) 2e+01) _returnvalue) (+ _returnvalue (* (Math|Vector|GetUpVector _boxs) 1e+02)) 5.0 "TraceTypeQuery3" false 0 "None"))
  (return _outhit))